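; Game instance for a 2D squirrel game that keeps pickup and level-won state across map loads and opens the game menu at startup.
; Init spawns a PickupSpawner fed by the PickupLocations array, then shows the menu with UI-only input and a mouse cursor.
; ExitLevel flags the matching entry as won if the level was won, reopens MainMap, and respawns pickups from that array after a short delay.
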(event `self.ReceiveInit`
  (bind _returnvalue (`GameplayStatics.GetPlayerController` 0))
  (bind _returnvalue_2 (`|SpawnActorFromClass` "/Game/Blueprints/Pickups/PickupSpawner.PickupSpawner_C" (`KismetMathLibrary.MakeTransform` (0.0 0.0 0.0)) "Undefined" "MultiplyWithRoot" null null))
  (`/Game/Blueprints/Pickups/PickupSpawner.SpawnPickups` _returnvalue_2 (`self.PickupLocations`))
  (`KismetSystemLibrary.Delay` 0.1)
  (bind _returnvalue_3 (`|CreateWidget` "/Game/Blueprints/Widgets/GameMenu.GameMenu_C"))
  (`UserWidget.AddToViewport` _returnvalue_3 0)
  (`WidgetBlueprintLibrary.SetInputMode_UIOnlyEx` _returnvalue _returnvalue_3 "DoNotLock" true)
  (set `PlayerController.bShowMouseCursor` true _returnvalue))

(event `RespawnPickups`
  (`KismetSystemLibrary.Delay` 0.2)
  (bind _returnvalue (`|SpawnActorFromClass` "/Game/Blueprints/Pickups/PickupSpawner.PickupSpawner_C" (`KismetMathLibrary.MakeTransform` (0.0 0.0 0.0)) "Undefined" "MultiplyWithRoot" null null))
  (`/Game/Blueprints/Pickups/PickupSpawner.SpawnPickups` _returnvalue (`self.PickupLocations`)))

(fn `Exit Level`
  (params (LevelName :type Name) (`LevelWon?` :type Boolean))
  (bind _pickuplocations (`self.PickupLocations`))
  (if `LevelWon?`
    (for (_array_element _array_index) (`self.PickupLocations`)
      (bind (_pickupgamemapname _location) (break `/Game/Structs/PickupLocationStruct` _array_element))
      (if (== _pickupgamemapname LevelName)
        (bind _structout (setmembers `/Game/Structs/PickupLocationStruct` :`StructRef` (`|GetArrayItem` _pickuplocations _array_index) :`PickupGameMapName` _pickupgamemapname :`Location` _location :`GameWon` true))
        (`KismetArrayLibrary.Array_Set` _pickuplocations _array_index _structout)
        (break))))
  (`GameplayStatics.OpenLevel` "MainMap")
  (`self.RespawnPickups`))

(fn `GetPickupLocations`
  (returns (NewParam :type "Array of /Game/Structs/PickupLocationStruct Structure"))
  (return (`self.PickupLocations`)))