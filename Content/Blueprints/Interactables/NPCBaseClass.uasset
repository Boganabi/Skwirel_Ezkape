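; Base class for interactable NPCs that randomly wander or idle and can open a dialogue screen.
; HandleMovement loops on a coin flip: AI move to a random point in a hardcoded world-space rectangle at fixed height, or wait a few seconds.
; Failed moves retry after a short delay.
; Interact shows a DialogueScreen fed by DialogueList, switches to UI-only input with cursor, and pauses the game.
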(event `self.ReceiveBeginPlay`
  (`parent.ReceiveBeginPlay`)
  (bind _wander (`self.GetRandomState`))
  (`self.HandleMovement` _wander))

(event `HandleMovement`
  (params (Wander :type Boolean))
  (if Wander
    (`AITask_MoveTo.AIMoveTo` (`AIBlueprintHelperLibrary.GetAIController` (`self.GetController`)) (`KismetMathLibrary.MakeVector` (`KismetMathLibrary.RandomFloatInRange` -1105.0 1478.0) (`KismetMathLibrary.RandomFloatInRange` -650.0 -64.0) 1222.0) null
      (:`OnRequestFailed`
        (`KismetSystemLibrary.Delay` 1.0)
        (`self.HandleMovement` true))
      (:`OnMoveFinished`
        (bind _wander (`self.GetRandomState` :!label _label))
        (`self.HandleMovement` _wander)))
    (else
      (`KismetSystemLibrary.Delay` (`KismetMathLibrary.RandomFloatInRange` 2.0 10.0))
      (goto _label))))

(fn `GetRandomState`
  (returns (Wander :type Boolean))
  (return (`KismetMathLibrary.RandomBool`)))

(fn `Interact`
  (bind _returnvalue (`GameplayStatics.GetPlayerController` 0))
  (`parent.Interact`)
  (bind _returnvalue_2 (`|CreateWidget` "/Game/Blueprints/Widgets/DialogueScreen.DialogueScreen_C"))
  (`/Game/Blueprints/Widgets/DialogueScreen.SetDialogueOptions` _returnvalue_2 (`self.DialogueList`))
  (`UserWidget.AddToViewport` _returnvalue_2 0)
  (`WidgetBlueprintLibrary.SetInputMode_UIOnlyEx` _returnvalue _returnvalue_2 "DoNotLock" true)
  (set `PlayerController.bShowMouseCursor` true _returnvalue)
  (`GameplayStatics.SetGamePaused` true))

(fn `UserConstructionScript`
  (`parent.UserConstructionScript`))