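; PlayerBP is the player character, a Paper2D flipbook sprite that walks, interacts with objects and opens the game menu.
; Axis inputs drive movement along vectors built from control pitch with zero yaw; left/right also picks the walk flipbook, defaulting to left at zero input.
; Interact calls the object stored through SetInteractingObject, if valid.
; OpenMenu creates a GameMenu widget, switches to UI-only input and shows the cursor.
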(event `InputAxis|LeftRightAxis`
  (params (AxisValue :type "Float (single-precision)"))
  ;[1 1 1] Input control
  (`self.AddMovementInput` (`KismetMathLibrary.GetRightVector` (`KismetMathLibrary.MakeRotator` 0.0 (.pitch (`self.GetControlRotation`)))) AxisValue)
  (`PaperFlipbookComponent.SetFlipbook` (`self.Sprite`) (select `bool` (> AxisValue 0.0) :`false` "/Game/Assets/Characters/WalkAnim/walkLeft.walkLeft" :`true` "/Game/Assets/Characters/WalkAnim/walkRight.walkRight" :!type "PaperFlipbook Object Reference")))

(event `InputAxis|UpDownAxis`
  (params (AxisValue :type "Float (single-precision)"))
  ;[1 1 1] Input control
  (`self.AddMovementInput` (`KismetMathLibrary.GetForwardVector` (`KismetMathLibrary.MakeRotator` 0.0 (.pitch (`self.GetControlRotation`)))) AxisValue))

(event `InputAction|OpenMenu`
  (params (Key :type "Key Structure"))
  (bind _returnvalue (`GameplayStatics.GetPlayerController` 0))
  (:`Pressed`
    (bind _returnvalue_2 (`|CreateWidget` "/Game/Blueprints/Widgets/GameMenu.GameMenu_C"))
    (`UserWidget.AddToViewport` _returnvalue_2 0)
    (`WidgetBlueprintLibrary.SetInputMode_UIOnlyEx` _returnvalue _returnvalue_2 "DoNotLock" true)
    (set `PlayerController.bShowMouseCursor` true _returnvalue)))

(event `InputAction|Interact`
  (params (Key :type "Key Structure"))
  (bind _interactingobject (`self.InteractingObject`))
  (:`Pressed`
    (`/Engine/EditorBlueprintResources/StandardMacros.IsValid` _interactingobject
      (:`Is Valid`
        (`/Game/Blueprints/Interactables/InteractableBaseBP.Interact` _interactingobject)))))

(fn `SetInteractingObject`
  (params (NewObject :type "/Game/Blueprints/Interactables/InteractableBaseBP Object Reference"))
  (set `self.InteractingObject` NewObject))

(fn `UserConstructionScript`)